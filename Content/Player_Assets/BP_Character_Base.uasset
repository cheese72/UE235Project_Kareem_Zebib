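; Base character Blueprint that manages weapon acquisition and switching, starting play with a grenade launcher.
; Acquiring spawns the weapon, makes it current, snaps it to its class-default mesh socket and starts a switch.
; Switching stores the pending weapon and plays a montage; SwitchHandNotify then sends the current weapon to inventory and puts the pending one in hand.
; A getter exposes the active weapon's idle and walk animations.
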(event Custom|Acquire_New_Weapon
  (params (Weapon_Class :type BP%20Weapon%20Base%20Class%20Reference))
  (bind _equip_socket_name (Utilities|GetClassDefaults Weapon_Class))
  (bind _self self)
  (bind _returnvalue (Game|SpawnActorfromClass Weapon_Class (Transformation|GetSocketTransform (Variables|Character|GetMesh) _equip_socket_name "RTS_World") "Undefined" "MultiplyWithRoot" _self _self))
  (bind _output_get (Variables|Default|SetCurrent_Active_Weapon _returnvalue))
  (Transformation|AttachComponentToComponent _output_get (Variables|Character|GetMesh) _equip_socket_name "SnapToTarget" "SnapToTarget" "SnapToTarget" true)
  (CallFunction|SwitchActiveWeaponto _returnvalue))

(event Custom|SwitchActiveWeaponTo
  (params (PendingNextWeapon :type BP%20Weapon%20Base%20Object%20Reference))
  (Variables|Default|SetPendingNextWeapon PendingNextWeapon)
  (Animation|Montage|PlayMontage (Variables|Character|GetMesh) "/Game/Animations/AS_Weapon_Switch_Montage.AS_Weapon_Switch_Montage"))

(event Custom|WeaponHandSwitchNotify)

(event Custom|SwitchHandNotify
  (Utilities|FlowControl|Sequence
    (:then_0
      (Utilities|IsValid (Variables|Default|GetCurrent_Active_Weapon)
        (:Is%20Valid
          (Default|WeaponInventory (Variables|Default|GetCurrent_Active_Weapon)))))
    (:then_1
      (bind _output_get (Variables|Default|SetCurrent_Active_Weapon (Variables|Default|GetPendingNextWeapon)))
      (Default|WeaponHand _output_get))))

(event EventBeginPlay
  (CallFunction|AcquireNewWeapon "/Game/Blueprints/Weapons/BP_Grenade_Launcher.BP_Grenade_Launcher_C"))

(event EventTick
  (params (DeltaSeconds :type Float%20%28single-precision%29)))

(event Collision|EventActorBeginOverlap
  (params (OtherActor :type Actor%20Object%20Reference)))

(fn ConstructionScript)

(fn GetActiveWeaponsAnims
  (bind _current_active_weapon (Variables|Default|GetCurrent_Active_Weapon))
  (return (Variables|/Game/Blueprints/Weapons/BP_Weapon_Base.BP_Weapon_Base_C|GetIdleAnim _current_active_weapon) (Variables|/Game/Blueprints/Weapons/BP_Weapon_Base.BP_Weapon_Base_C|GetWalkAnim _current_active_weapon)))