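; Base weapon Blueprint that handles showing or hiding the weapon and starting its attack animation.
; WeaponHand and WeaponInventory toggle the root component's visibility without propagating to children.
; Attack triggers the attack animation event, which casts the owner to BP_Character_Base, plays AttackAnim on its mesh and prints the montage name.
; The attack commit notify event is an empty stub, and the file contains no damage logic.
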(event Custom|WeaponInventory
  (Rendering|SetVisibility (Variables|Default|GetDefaultSceneRoot) false false))

(event Custom|WeaponHand
  (Rendering|SetVisibility (Variables|Default|GetDefaultSceneRoot) true false))

(event Custom|Play_attack_anim
  (bind _attack_anim (Variables|Default|GetAttack%20Anim))
  ;[0.15 0.15 0.15 0.5] Attacking stuff
  (bind _asbp_character_base (Utilities|Casting|CastToBP_Character_Base (Components|GetOwner)))
  (Animation|Montage|PlayMontage (Variables|/Script/Engine.Character|GetMesh _asbp_character_base) _attack_anim
    (:then
      (Development|PrintString (Utilities|GetDisplayName _attack_anim)))))

(event Custom|Attack
  ;[0.15 0.15 0.15 0.5] Attacking stuff
  (CallFunction|PlayAttackAnim))

(event Custom|Commit_attack_Anim_Notify
  ;[0.15 0.15 0.15 0.5] Attacking stuff
)

(event EventBeginPlay)

(event Collision|EventActorBeginOverlap
  (params (OtherActor :type Actor%20Object%20Reference)))

(event EventTick
  (params (DeltaSeconds :type Float%20%28single-precision%29)))

(fn ConstructionScript)