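; BP_Triggerable is a generic trigger actor that reacts when characters enter or leave its Trigger component.
; Begin and end overlaps pass through CharacterCheck, which accepts only actors whose class derives from Character.
; Accepted actors are forwarded to the custom events Overlap_THIS and Unoverlapped_THIS, which here only print the actor's display name.
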(event OnComponentBeginOverlap(Trigger)
  (params (OverlappedComponent :type Primitive%20Component%20Object%20Reference) (OtherActor :type Actor%20Object%20Reference) (OtherComp :type Primitive%20Component%20Object%20Reference) (OtherBodyIndex :type Integer) (bFromSweep :type Boolean) (SweepResult :type Hit%20Result%20Structure%20%28by%20ref%29))
  (bind _returnvalue (CallFunction|CharacterCheck OtherActor))
  (if _returnvalue
    (CallFunction|OverlapTHIS OtherActor)))

(event OnComponentEndOverlap(Trigger)
  (params (OverlappedComponent :type Primitive%20Component%20Object%20Reference) (OtherActor :type Actor%20Object%20Reference) (OtherComp :type Primitive%20Component%20Object%20Reference) (OtherBodyIndex :type Integer))
  (bind _returnvalue (CallFunction|CharacterCheck OtherActor))
  (if _returnvalue
    (CallFunction|UnoverlappedTHIS OtherActor)))

(event Custom|Overlap_THIS
  (params (Other%20Actor :type Actor%20Object%20Reference))
  (Development|PrintString (Utilities|GetDisplayName Other%20Actor)))

(event Custom|Unoverlapped_THIS
  (params (Other%20Actor :type Actor%20Object%20Reference))
  (Development|PrintString (Utilities|GetDisplayName Other%20Actor)))

(event EventBeginPlay)

(event Collision|EventActorBeginOverlap
  (params (OtherActor :type Actor%20Object%20Reference)))

(event EventTick
  (params (DeltaSeconds :type Float%20%28single-precision%29)))

(fn ConstructionScript)

(fn CharacterCheck
  (params (Object :type Object%20Object%20Reference))
  (return (Utilities|ClassIsChildOf (Utilities|GetClass Object) "/Script/Engine.Character")))